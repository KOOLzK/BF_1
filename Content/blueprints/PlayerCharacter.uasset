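; Player character Blueprint that adds keyboard shortcuts for dying and leaving the level.
; K calls PressToDie, while O and Escape both open the MainMenu level; BeginPlay, overlap and Tick do nothing.
; Unconnected leftovers include a one-shot death camera turn, which feeds a look-at rotation toward DeathTrun into DeathLook, and a quit-game call.
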(event EventBeginPlay)

(event Collision|EventActorBeginOverlap
  (params (OtherActor :type Actor%20Object%20Reference)))

(event EventTick
  (params (DeltaSeconds :type Float%20%28single-precision%29)))

(event Input|KeyboardEvents|Escape
  (params (Key :type Key%20Structure :default "AnyKey"))
  (:Pressed
    (Game|OpenLevel(byName) "MainMenu")))

(event Input|KeyboardEvents|O
  (params (Key :type Key%20Structure :default "AnyKey"))
  (:Pressed
    (Game|OpenLevel(byName) "MainMenu")))

(event Input|KeyboardEvents|K
  (params (Key :type Key%20Structure :default "AnyKey"))
  (:Pressed
    (Class|PlayerCharacter|PresstoDie)))

(fn ConstructionScript)