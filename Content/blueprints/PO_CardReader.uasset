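; Card reader object that flips its state when the saved key card level meets or exceeds its required level.
; Its StringToInt event loads level.txt, searches for the KeyLevel tag and parses the single digit after the following equals sign.
; That value is compared with GetRequiredLevel, and BPFlipState fires on equal or greater.
; The event's String input is unused in the live path, and the SetCardLevel calls are disconnected.
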(event Custom|StringToInt
  (params (String :type String))
  (bind _savetexta (Class|RWTxtFile|LoadTxt "level.txt"))
  (bind _output_get (Variables|Default|SetCardWord "KeyLevel"))
  (if (Utilities|Enum|Equal(Enum) (Utilities|String|GetSubstring _savetexta (Utilities|String|FindSubstring _savetexta _output_get) (Utilities|String|Len _output_get)) _output_get)
    (bind _returnvalue (Class|PGCardReader|GetRequiredLevel))
    (Math|Integer|CompareInt (Math|Conversions|ToInteger(Byte) (Utilities|String|GetSubstring _savetexta (+ (Utilities|String|FindSubstring _savetexta "=" false false (Utilities|String|FindSubstring _savetexta _output_get)) 1))) _returnvalue
      (:>
        _)
      (:==
        _))
    (Class|PGCardReader|BPFlipState)))

(event EventBeginPlay)

(event Collision|EventActorBeginOverlap
  (params (OtherActor :type Actor%20Object%20Reference)))

(event EventTick
  (params (DeltaSeconds :type Float%20%28single-precision%29)))

(fn ConstructionScript)